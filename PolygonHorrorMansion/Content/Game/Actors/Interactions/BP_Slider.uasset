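; BP_Slider is an interactable actor whose mesh slides open and closed, such as a drawer or sliding panel.
; Each interaction calls the parent handler, then a FlipFlop alternates the Open/Close event, which plays or reverses a Timeline.
; The Timeline lerps the mesh's relative location from zero to an offset on local Y, set by ZValue despite its name, without sweeping.
; Hover and unhover events are empty.
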(event Custom|Open/Close
  (params (IsOpen :type Boolean))
  (if IsOpen
    (bind _newtrack_0 (Timeline|Timeline Play)
      (:Update
        (Transformation|SetRelativeLocation (Variables|Default|GetStaticMesh) (Math|Vector|Lerp(Vector) "0, 0, 0" (Math|Vector|MakeVector 0.0 (Variables|Default|GetZ%20Value) 0.0) _newtrack_0) false true)))
    (else
      (Timeline|Timeline Reverse))))

(event EventBeginPlay
  (|CallParentFunction) ; This node is disabled and will not be called.\nDrag off pins to build functionality.
)

(event Collision|EventActorBeginOverlap
  (params (OtherActor :type Actor%20Object%20Reference))
  (|CallParentFunction OtherActor) ; This node is disabled and will not be called.\nDrag off pins to build functionality.
)

(event EventTick
  (params (DeltaSeconds :type Float%20%28single-precision%29))
  (|CallParentFunction DeltaSeconds) ; This node is disabled and will not be called.\nDrag off pins to build functionality.
)

(event EventEventInteract
  (params (Character :type BP%20Character%20Object%20Reference))
  (|CallParentFunction Character)
  (Utilities|FlowControl|FlipFlop
    (:A
      (CallFunction|Open/Close true))
    (:B
      (CallFunction|Open/Close false))))

(event EventEventHover)

(event EventEventUnHover)

(fn ConstructionScript
  (|CallParentFunction))