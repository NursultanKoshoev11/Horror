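; Interactable actor that swings its static mesh open and closed by 90 degrees, as for a door or hatch.
; Each interaction calls the parent handler, then a FlipFlop alternates the Open/Close event between playing and reversing a timeline.
; The timeline drives a rotator lerp on the mesh's relative rotation, with IsReverse flipping the swing direction.
; Hover and unhover events only print debug strings.
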(event Custom|Open/Close
  (params (IsOpen :type Boolean))
  (bind _output_get (Variables|Default|SetIs%20Open IsOpen))
  (if _output_get
    (bind _newtrack_0 (Timeline|OpenClose Play)
      (:Update
        (Transformation|SetRelativeRotation (Variables|Default|GetStaticMesh) (Math|Rotator|Lerp(Rotator) "0, 0, 0" (select (Variables|Setting|GetIsReverse) "0.000000,90.000000,0.000000" "0.000000,-90.000000,0.000000") _newtrack_0 true) false false)))
    (else
      (Timeline|OpenClose Reverse))))

(event EventBeginPlay)

(event Collision|EventActorBeginOverlap
  (params (OtherActor :type Actor%20Object%20Reference)))

(event EventTick
  (params (DeltaSeconds :type Float%20%28single-precision%29)))

(event EventEventInteract
  (params (Character :type BP%20Character%20Object%20Reference))
  (|CallParentFunction Character)
  (Utilities|FlowControl|FlipFlop
    (:A
      (CallFunction|Open/Close true))
    (:B
      (CallFunction|Open/Close false))))

(event EventEventHover
  (Development|PrintString "Hover"))

(event EventEventUnHover
  (Development|PrintString "UnHover"))

(fn ConstructionScript)