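; BP_Moveble is an interactable actor whose static mesh briefly rotates when interacted with.
; EventInteract calls StartTimer, which plays a Timeline from the start on each trigger.
; The Timeline's track drives a shortest-path rotator lerp from zero to a slight single-axis tilt, and the mesh snaps back to zero relative rotation when it finishes.
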(event Custom|StartTimer
  (bind _newtrack_0 (Timeline|Timeline PlayFromStart)
    (:Update
      (Transformation|SetRelativeRotation (Variables|Default|GetStaticMesh) (Math|Rotator|Lerp(Rotator) "0.000000,0.000000,0.000000" "0.000000,0.000000,-10.000000" _newtrack_0 true) false false))
    (:Finished
      (Transformation|SetRelativeRotation (Variables|Default|GetStaticMesh) "0, 0, 0" false false))))

(event EventBeginPlay
  (|CallParentFunction) ; This node is disabled and will not be called.\nDrag off pins to build functionality.
)

(event Collision|EventActorBeginOverlap
  (params (OtherActor :type Actor%20Object%20Reference))
  (|CallParentFunction OtherActor) ; This node is disabled and will not be called.\nDrag off pins to build functionality.
)

(event EventTick
  (params (DeltaSeconds :type Float%20%28single-precision%29))
  (|CallParentFunction DeltaSeconds) ; This node is disabled and will not be called.\nDrag off pins to build functionality.
)

(event EventEventInteract
  (CallFunction|StartTimer))

(fn ConstructionScript
  (|CallParentFunction))