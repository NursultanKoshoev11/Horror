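; BP_Key is an interactable key pickup that increments the game's key progress when a character interacts with it.
; It extends a parent interaction event, then uses an authority check so only the server calls AddKey on BP_GameGM.
; The key actor destroys itself after the interaction, and it has no other active logic.
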(event EventBeginPlay
  (|CallParentFunction) ; This node is disabled and will not be called.\nDrag off pins to build functionality.
)

(event Collision|EventActorBeginOverlap
  (params (OtherActor :type Actor%20Object%20Reference))
  (|CallParentFunction OtherActor) ; This node is disabled and will not be called.\nDrag off pins to build functionality.
)

(event EventTick
  (params (DeltaSeconds :type Float%20%28single-precision%29))
  (|CallParentFunction DeltaSeconds) ; This node is disabled and will not be called.\nDrag off pins to build functionality.
)

(event EventEventInteract
  (params (Character :type BP%20Character%20Object%20Reference))
  (|CallParentFunction Character)
  (Networking|SwitchHasAuthority
    (:Authority
      (bind _asbp_game_gm (Utilities|Casting|CastToBP_GameGM (Game|GetGameMode))
        (:then
          (Default|AddKey _asbp_game_gm))
        (:CastFailed
          _)))
    (:Remote
      _))
  (Actor|DestroyActor))

(fn ConstructionScript
  (|CallParentFunction))