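; BP_Overlap is an overlap volume that gives overlapping BP_Characters a tag while none of its linked door actors is open.
; Each begin overlap starts a looping half-second timer that checks the doors and calls OnTagAdd or OnTagRemove on every character inside.
; A leaving character loses the tag, and the last stored timer handle is cleared once no characters remain.
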(event Custom|CustomEvent
  (if (CallFunction|CheckActors)
    (bind _output_get (Variables|Default|SetOverlapping%20Actors (Collision|GetOverlappingActors "/Game/Game/Character/BP_Character.BP_Character_C" :!class /Script/Engine.Actor)))
    (for _array_element _output_get
      (Default|OnTagRemove _array_element (Variables|Default|GetAddTag)))
    (else
      (bind _output_get_2 (Variables|Default|SetOverlapping%20Actors (Collision|GetOverlappingActors "/Game/Game/Character/BP_Character.BP_Character_C" :!class /Script/Engine.Actor)))
      (for _array_element_2 _output_get_2
        (Default|OnTagAdd _array_element_2 (Variables|Default|GetAddTag))))))

(event Collision|EventActorBeginOverlap
  (params (OtherActor :type Actor%20Object%20Reference))
  (bind _returnvalue (Utilities|Time|SetTimerbyEvent (delegate Custom|CustomEvent) 0.5 true))
  (Variables|Default|SetTimerHandle _returnvalue))

(event Collision|EventActorEndOverlap
  (params (OtherActor :type Actor%20Object%20Reference))
  (bind _asbp_character (Utilities|Casting|CastToBP_Character OtherActor))
  (Default|OnTagRemove _asbp_character (Variables|Default|GetAddTag))
  (if (Utilities|Array|IsEmpty (Collision|GetOverlappingActors "/Game/Game/Character/BP_Character.BP_Character_C" :!class /Script/Engine.Actor))
    (Utilities|Time|ClearandInvalidateTimerbyHandle (Variables|Default|GetTimerHandle))))

(fn ConstructionScript)

(fn CheckActors
  (for _array_element (Variables|Default|GetDoorActors)
    (if (Variables|/Game/Game/Actors/Interactions/BP_OpenClose.BP_OpenClose_C|GetIs%20Open _array_element)
      (return true)))
  (return false))