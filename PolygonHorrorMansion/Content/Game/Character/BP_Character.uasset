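; BP_Character is a player character with Enhanced Input movement, crouch, jump and sprint.
; Sprint switches walk speed through a server event.
; PlaySound, limited to player pawn 0, prints a debug string, plays a footstep through the sound subsystem at the left foot, and has the server emit pawn noise there.
; Tag events maintain a unique Tags list, with additions also calling OnHide.
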(event Custom|OnTagAdd
  (params (NewItem :type Name%20%28by%20ref%29))
  (Utilities|Array|AddUnique (Variables|Actor|GetTags) NewItem)
  (Default|CallOnHide))

(event Custom|Server%20|%20Noice
  (params (NoiseLocation :type Vector%20%28by%20ref%29))
  (Class|PawnNoiseEmitterComponent|MakeNoise (Variables|Default|GetPawnNoiseEmitter) self 1.0 NoiseLocation))

(event Custom|Server%20|%20SetWalkSpeed
  (params (Max%20Walk%20Speed :type Float%20%28single-precision%29))
  ;[0.15 0.15 0.15 0.5] Comment
  (Variables|/Script/Engine.CharacterMovementComponent|SetMaxWalkSpeed (Variables|Character|GetCharacterMovement) Max%20Walk%20Speed))

(event Custom|OnTagRemove
  (params (Item :type Name%20%28by%20ref%29))
  (Utilities|Array|RemoveItem (Variables|Actor|GetTags) Item))

(event Custom|PlaySound
  (params (SoundValue :type Float%20%28double-precision%29) (NoiceValue :type Float%20%28double-precision%29))
  (bind _mesh (Variables|Character|GetMesh))
  (bind _returnvalue (Transformation|GetSocketLocation _mesh "foot_l"))
  (if (== (Game|Player|GetPlayerPawn 0) self)
    (Development|PrintString "Hello")
    (Class|SoundSubsystem|PlaySound (Subsystems|GetSoundSubsystem) "/Game/Game/Sounds/Footstep/MSS_Footstep.MSS_Footstep" _returnvalue NoiceValue)
    (CallFunction|Server|Noice _returnvalue)))

(event Input|EnhancedActionEvents|EnhancedInputActionIA_MoveFB
  (params (ActionValue :type Float%20%28double-precision%29) (ElapsedSeconds :type Float%20%28double-precision%29) (TriggeredSeconds :type Float%20%28double-precision%29) (InputAction :type Input%20Action%20Object%20Reference :default "/Game/Game/Input/Actions/IA_MoveFB.IA_MoveFB"))
  ;[0.15 0.15 0.15 0.5] Comment
  (Pawn|Input|AddMovementInput (Transformation|GetActorForwardVector) ActionValue false))

(event Input|EnhancedActionEvents|EnhancedInputActionIA_MoveRL
  (params (ActionValue :type Float%20%28double-precision%29) (ElapsedSeconds :type Float%20%28double-precision%29) (TriggeredSeconds :type Float%20%28double-precision%29) (InputAction :type Input%20Action%20Object%20Reference :default "/Game/Game/Input/Actions/IA_MoveRL.IA_MoveRL"))
  ;[0.15 0.15 0.15 0.5] Comment
  (Pawn|Input|AddMovementInput (Transformation|GetActorRightVector) ActionValue false))

(event Input|EnhancedActionEvents|EnhancedInputActionIA_Crouch
  (params (ActionValue :type Boolean) (ElapsedSeconds :type Float%20%28double-precision%29) (TriggeredSeconds :type Float%20%28double-precision%29) (InputAction :type Input%20Action%20Object%20Reference :default "/Game/Game/Input/Actions/IA_Crouch.IA_Crouch"))
  ;[0.15 0.15 0.15 0.5] Comment
  (:Started
    (Character|Crouch))
  (:Completed
    (Character|UnCrouch)))

(event Input|EnhancedActionEvents|EnhancedInputActionIA_Jump
  (params (ActionValue :type Boolean) (ElapsedSeconds :type Float%20%28double-precision%29) (TriggeredSeconds :type Float%20%28double-precision%29) (InputAction :type Input%20Action%20Object%20Reference :default "/Game/Game/Input/Actions/IA_Jump.IA_Jump"))
  ;[0.15 0.15 0.15 0.5] Comment
  (:Started
    (Character|Jump))
  (:Completed
    (Character|StopJumping)))

(event Input|EnhancedActionEvents|EnhancedInputActionIA_Sprint
  (params (ActionValue :type Boolean) (ElapsedSeconds :type Float%20%28double-precision%29) (TriggeredSeconds :type Float%20%28double-precision%29) (InputAction :type Input%20Action%20Object%20Reference :default "/Game/Game/Input/Actions/IA_Sprint.IA_Sprint"))
  ;[0.15 0.15 0.15 0.5] Comment
  (:Started
    (CallFunction|Server|SetWalkSpeed 4e+02))
  (:Completed
    (CallFunction|Server|SetWalkSpeed 1.8e+02)))

(event EventBeginPlay)

(fn ConstructionScript)