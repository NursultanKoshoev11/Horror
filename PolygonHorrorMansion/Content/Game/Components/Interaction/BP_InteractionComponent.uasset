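; Player character component that lets the player highlight and use interactable actors in a networked game.
; On non-authority instances, a looping timer line-traces from the view point, toggling hover events, stencil outline, prompt widget and controller state on BP_BaseInteraction hits.
; The interact input sends the focused actor, or HitComponent if valid (never assigned here), through server-to-multicast events and plays a sound.
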(event Custom|Update
  (bind _client___controller (Variables|Default|GetClient%20|%20Controller))
  (bind (_location _rotation) (Pawn|GetPlayerViewPoint _client___controller))
  (bind (_outhit _returnvalue) (Collision|LineTraceByChannel _location (+ _location (* (Math|Vector|GetForwardVector _rotation) 2e+02)) "TraceTypeQuery1" false (Utilities|Array|MakeArray (Variables|Default|GetClient%20|%20Character)) "None"))
  (if _returnvalue
    (if (!= (Variables|Default|GetActor) (.HitActor (Collision|BreakHitResult _outhit)))
      (CallFunction|Disable)
      (bind _asbp_base_interaction (Utilities|Casting|CastToBP_BaseInteraction (.HitActor (Collision|BreakHitResult _outhit))))
      (bind _output_get (Variables|Default|SetActor _asbp_base_interaction))
      (Default|EventHover _output_get)
      (Default|SetInteracted (Variables|Default|GetClient%20|%20Controller) true)
      (Rendering|SetRenderCustomDepth (Variables|/Game/Game/Components/Interaction/BP_BaseInteraction.BP_BaseInteraction_C|GetStaticMesh (Variables|Default|GetActor)) true)
      (Rendering|SetCustomDepthStencilValue (Variables|/Game/Game/Components/Interaction/BP_BaseInteraction.BP_BaseInteraction_C|GetStaticMesh (Variables|Default|GetActor)) 1)
      (Components|Activation|Activate (Variables|/Game/Game/Components/Interaction/BP_BaseInteraction.BP_BaseInteraction_C|GetBP_InteractionWidgetComponent (Variables|Default|GetActor)) false))
    (else
      (CallFunction|Disable))))

(event Custom|Server%20|%20Interact
  (params (Target :type BP%20Base%20Interaction%20Object%20Reference) (Character :type BP%20Character%20Object%20Reference))
  ;[0.15 0.15 0.15 0.5] Comment
  (CallFunction|Multi|Interact Target Character))

(event Custom|Multi%20|%20Interact
  (params (Target :type BP%20Base%20Interaction%20Object%20Reference) (Character :type BP%20Character%20Object%20Reference))
  ;[0.15 0.15 0.15 0.5] Comment
  (Default|EventInteract Target Character))

(event Custom|Server%20|%20InteractComponent
  (params (Target :type Object%20Object%20Reference) (Character :type BP%20Character%20Object%20Reference))
  ;[0.15 0.15 0.15 0.5] Comment
  (CallFunction|Multi|InteractComponent Target Character))

(event Custom|Multi%20|%20InteractComponent
  (params (Target :type Object%20Object%20Reference) (Character :type BP%20Character%20Object%20Reference))
  ;[0.15 0.15 0.15 0.5] Comment
  (Class|BPIInteraction|OnInteract(Message) Target Character))

(event Input|EnhancedActionEvents|EnhancedInputActionIA_Interact
  (params (ActionValue :type Boolean) (ElapsedSeconds :type Float%20%28double-precision%29) (TriggeredSeconds :type Float%20%28double-precision%29) (InputAction :type Input%20Action%20Object%20Reference :default "/Game/Game/Input/Actions/IA_Interact.IA_Interact"))
  (bind _hit_component (Variables|Default|GetHit%20Component))
  (bind _actor (Variables|Default|GetActor))
  (:Started
    (Utilities|IsValid _hit_component
      (:Is%20Valid
        (CallFunction|Server|InteractComponent _hit_component (Variables|Default|GetClient%20|%20Character)))
      (:Is%20Not%20Valid
        (Utilities|IsValid _actor
          (:Is%20Valid
            (CallFunction|Server|Interact _actor (Variables|Default|GetClient%20|%20Character))))))
    (Class|SoundSubsystem|PlaySound (Subsystems|GetSoundSubsystem) 0 "0, 0, 0" 0.1)))

(event EventBeginPlay
  (Networking|SwitchHasAuthority
    (:Remote
      (bind _asbp_character (Utilities|Casting|CastToBP_Character (Components|GetOwner)))
      (Variables|Default|SetClient%20|%20Character _asbp_character)
      (bind _asbp_game_player_controller (Utilities|Casting|CastToBP_GamePlayerController (Pawn|GetController (Variables|Default|GetClient%20|%20Character))))
      (Variables|Default|SetClient%20|%20Controller _asbp_game_player_controller)
      (bind _returnvalue (Utilities|Time|SetTimerbyEvent (delegate Custom|Update) 0.1 true))
      (Variables|Default|SetTimerHandle _returnvalue))))

(event EventEndPlay
  (params (EndPlayReason :type EEndPlayReason%20Enum :default "Destroyed"))
  (if (Utilities|Time|IsValidTimerHandle (Variables|Default|GetTimerHandle))
    (Utilities|Time|ClearandInvalidateTimerbyHandle (Variables|Default|GetTimerHandle))))

(fn Disable
  (Default|SetInteracted (Variables|Default|GetClient%20|%20Controller) false)
  (Utilities|IsValid (Variables|Default|GetActor)
    (:Is%20Valid
      (Default|EventUnHover (Variables|Default|GetActor))
      (Components|Activation|Deactivate (Variables|/Game/Game/Components/Interaction/BP_BaseInteraction.BP_BaseInteraction_C|GetBP_InteractionWidgetComponent (Variables|Default|GetActor)))
      (Rendering|SetRenderCustomDepth (Variables|/Game/Game/Components/Interaction/BP_BaseInteraction.BP_BaseInteraction_C|GetStaticMesh (Variables|Default|GetActor)) false))
    (:Is%20Not%20Valid
      _))
  (Variables|Default|SetActor 0))