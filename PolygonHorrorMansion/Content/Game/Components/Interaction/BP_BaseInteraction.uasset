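; BP_BaseInteraction is a base actor for interactables, with empty hover and unhover events and a shared interact response.
; On BeginPlay, it registers itself with the spawn subsystem when flagged as a spawn key.
; On interact, the authority makes noise at the actor's location through the character's PawnNoiseEmitter, while remotes only play the interact sound there.
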(event Custom|EventUnHover)

(event Custom|EventHover)

(event Custom|EventInteract
  (params (Character :type BP%20Character%20Object%20Reference))
  (Networking|SwitchHasAuthority
    (:Authority
      (Class|PawnNoiseEmitterComponent|MakeNoise (Variables|/Game/Game/Character/BP_Character.BP_Character_C|GetPawnNoiseEmitter Character) Character 1.0 (Transformation|GetActorLocation)))
    (:Remote
      (Audio|PlaySoundatLocation (Variables|Sound|GetInteractSound) (Transformation|GetActorLocation) "0, 0, 0" 1.0 1.0 0.0 0 0 0 0))))

(event EventBeginPlay
  (if (Variables|Default|GetIsSpawnKey)
    (Class|SpawnSubsystem|SetActor (Subsystems|GetSpawnSubsystem) self)))

(fn ConstructionScript)