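; Server-driven hunter AI that activates on the game mode's High event and walks back to its start location on Low.
; While active, a looping timer picks a target from sighted actors not tagged CharacterHide, and heard noises become move destinations when it has no enemy.
; Targets feed the Blackboard, and a proximity timer tags caught characters' PlayerState Dead and destroys them.
; A character's Hide event clears the target.
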(event OnHearNoise(PawnSensing)
  (params (Instigator :type Pawn%20Object%20Reference) (Location :type Vector%20%28by%20ref%29 :default "0, 0, 0") (Volume :type Float%20%28single-precision%29))
  ;[0.15 0.15 0.15 0.5] Comment
  (if (Variables|Default|GetIsHightActive)
    (Utilities|IsValid (AI|Components|Blackboard|GetValueasObject (Variables|Default|GetBlackboard) (Variables|Keys|GetEnemyKey))
      (:Is%20Not%20Valid
        (if (not (Variables|Default|GetIsMoveving))
          (Variables|Default|SetIsMoveving true)
          (AI|Components|Blackboard|SetValueasVector (Variables|Default|GetBlackboard) (Variables|Keys|GetLocationKey) Location)
          (AI|AIMoveTo self Location 0 5e+01 false
            (:OnSuccess
              _)
            (:OnFail
              _))
          (Variables|Default|SetIsMoveving false)
          (AI|Components|Blackboard|ClearValue (Variables|Default|GetBlackboard) (Variables|Keys|GetLocationKey)))))))

(event Custom|CharacterHide
  ;[0.15 0.15 0.15 0.5] Comment
  (EventDispatchers|UnbindEventfromOnHide (Variables|Default|GetAs%20BP%20Character) (delegate Custom|CharacterHide))
  (AI|Components|Blackboard|ClearValue (Variables|Default|GetBlackboard) (Variables|Keys|GetEnemyKey))
  (Variables|Default|SetTargetActor 0)
  (Utilities|Time|ClearandInvalidateTimerbyHandle (Variables|Default|GetTimerHandle))
  (AI|Components|Blackboard|ClearValue (Variables|Default|GetBlackboard) (Variables|Keys|GetLocationKey)))

(event Custom|CheckActor
  ;[0.15 0.15 0.15 0.5] Comment
  (Utilities|IsValid (Variables|Default|GetAs%20BP%20Character)
    (:Is%20Valid
      (if (Utilities|Operators|EqualEqual (Transformation|GetActorLocation (Variables|Default|GetAs%20BP%20Character)) (Transformation|GetActorLocation) 1e+02)
        (CallFunction|CharacterHide)
        (Utilities|Array|AddUnique (Variables|/Script/Engine.Actor|GetTags (Variables|/Script/Engine.Pawn|GetPlayerState (Variables|Default|GetAs%20BP%20Character))) "Dead")
        (Actor|DestroyActor (Variables|Default|GetAs%20BP%20Character))
        (CallFunction|RandomLocation)))))

(event Custom|Hight
  (Variables|Default|SetIsHightActive true)
  (bind _returnvalue (Utilities|Time|SetTimerbyEvent (delegate Custom|Update) 0.1 true))
  (Variables|Default|SetCheckTimer _returnvalue))

(event Custom|Low
  (AI|Components|Blackboard|SetValueasVector (Variables|Default|GetBlackboard) (Variables|Keys|GetLocationKey) (Variables|Default|GetStartLocation))
  (Utilities|Time|ClearandInvalidateTimerbyHandle (Variables|Default|GetRandomTimer))
  (AI|AIMoveTo self (Variables|Default|GetStartLocation) 0 5e+01 false
    (:OnSuccess
      (Variables|Default|SetIsHightActive false)
      (AI|Components|Blackboard|ClearValue (Variables|Default|GetBlackboard) (Variables|Keys|GetLocationKey))
      (Utilities|Time|ClearandInvalidateTimerbyHandle (Variables|Default|GetCheckTimer)))))

(event Custom|UpdatePerception
  (params (Actor :type Actor%20Object%20Reference))
  (if (Variables|Default|GetIsHightActive)
    (Utilities|IsValid (Variables|Default|GetAs%20BP%20Character)
      (:Is%20Valid
        (CallFunction|CharacterHide))
      (:Is%20Not%20Valid
        _))
    (AI|Components|Blackboard|SetValueasObject (Variables|Default|GetBlackboard) (Variables|Keys|GetEnemyKey) Actor)
    (Variables|Default|SetTargetActor Actor)
    (bind _asbp_character (Utilities|Casting|CastToBP_Character Actor))
    (bind _output_get (Variables|Default|SetAs%20BP%20Character _asbp_character))
    (EventDispatchers|BindEventtoOnHide _output_get (delegate Custom|CharacterHide))
    (bind _returnvalue (Utilities|Time|SetTimerbyEvent (delegate Custom|CheckActor) 0.1 true))
    (Variables|Default|SetTimerHandle _returnvalue)))

(event Custom|RandomLocation
  (bind _returnvalue (Utilities|Time|SetTimerbyEvent (delegate Custom|CustomEvent) 2.0))
  (Variables|Default|SetRandomTimer _returnvalue))

(event Custom|CustomEvent
  (if (not (or (Utilities|Operators|EqualEqual :A (AI|Components|Blackboard|GetValueasVector (Variables|Default|GetBlackboard) (Variables|Keys|GetLocationKey))) (Utilities|IsValid (AI|Components|Blackboard|GetValueasObject (Variables|Default|GetBlackboard) (Variables|Keys|GetEnemyKey)))))
    (bind _randomlocation (Class|NavigationSystemV1|GetRandomLocationinNavigableRadius (Transformation|GetActorLocation) 1e+03 0 0))
    (AI|AIMoveTo self _randomlocation 0 5e+01 false
      (:OnSuccess
        (CallFunction|RandomLocation)))))

(event Custom|Update
  (CallFunction|CheckActors)
  (if (not (== (Variables|Default|GetTargetActor) (Variables|Default|GetAs%20BP%20Character)))
    (CallFunction|UpdatePerception (Variables|Default|GetTargetActor))))

(event EventBeginPlay
  (Networking|SwitchHasAuthority
    (:Authority
      (Variables|Default|SetStartLocation (Transformation|GetActorLocation))
      (Variables|Default|SetBlackboard (AI|GetBlackboard 0))
      (Variables|Default|SetAIController (AI|GetAIController self))
      (bind _asbp_game_gm (Utilities|Casting|CastToBP_GameGM (Game|GetGameMode)))
      (Variables|Default|SetAs%20BP%20Game%20GM _asbp_game_gm)
      (EventDispatchers|BindEventtoOnHightValue (Variables|Default|GetAs%20BP%20Game%20GM) (delegate Custom|Hight))
      (EventDispatchers|BindEventtoOnLowValue (Variables|Default|GetAs%20BP%20Game%20GM) (delegate Custom|Low)))))

(fn ConstructionScript)

(fn CheckActors
  (bind _output_get (LocalVariables|SetLocalArray (Class|AIPerceptionComponent|GetCurrentlyPerceivedActors (Variables|Default|GetAIPerception) "/Script/AIModule.AISense_Sight")))
  (for _array_element _output_get
    (if (not (Actor|ActorHasTag _array_element "CharacterHide"))
      (Utilities|IsValid (Variables|Default|GetTargetActor)
        (:Is%20Valid
          (if (> (LocalVariables|GetLocalDistance) (Transformation|GetDistanceTo _array_element self))
            (LocalVariables|SetLocalDistance (Transformation|GetDistanceTo _array_element self) :!label _label)
            (Variables|Default|SetTargetActor _array_element)))
        (:Is%20Not%20Valid
          (goto _label)))))
  (AI|Components|Blackboard|SetValueasObject (Variables|Default|GetBlackboard) (Variables|Keys|GetEnemyKey) (Variables|Default|GetTargetActor)))