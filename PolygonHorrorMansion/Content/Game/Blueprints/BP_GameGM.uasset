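; Game mode for a key-hunt match, won by collecting enough keys before the countdown expires.
; A shared audio value rises on input and decays on a timer, broadcasting updates and high/low events with hysteresis.
; Each login registers with the game state; the first also starts the countdown and, after a short delay, spawns five keys.
; Keys attach to free, key-enabled interaction actors from the spawn subsystem, probed from a random index.
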(event Custom|Time
  (bind _result (Math|Integer|DecrementInt (Variables|Default|GetGameTime))
    (:%20%20
      (if (<= _result 0)
        (Default|CallOnGameEnd false)
        (else
          (Default|CallOnTimeUpdate (Variables|Default|GetGameTime)))))))

(event Custom|AddKey
  (bind _currentkeys (Variables|Default|GetCurrentKeys))
  (bind _result (Math|Integer|IncrementInt _currentkeys)
    (:%20%20
      (Default|CallOnUpdateKey _currentkeys)
      (if (== _result (Variables|Default|GetKeyCountForWin))
        (Default|CallOnGameEnd true)))))

(event Custom|SetValue
  (params (AudioValue :type Float%20%28double-precision%29))
  ;[0.15 0.15 0.15 0.5] Comment
  (bind _output_get (Variables|Default|SetAudioValue (Math|Float|Clamp(Float) (+ AudioValue (Variables|Default|GetAudioValue)))))
  (Default|CallOnValueUpdate _output_get))

(event Custom|UpdateValue
  (Default|CallOnValueUpdate (Variables|Default|GetAudioValue)))

(event Custom|Update
  (Variables|Default|SetAudioValue (Math|Float|Clamp(Float) (- (Variables|Default|GetAudioValue) 0.005)))
  (if (> (Variables|Default|GetAudioValue) 0.8)
    (if (not (Variables|Default|GetIsHightActive))
      (Default|CallOnHightValue)
      (Variables|Default|SetIsHightActive true))
    (elif (and (< (Variables|Default|GetAudioValue) 0.3) (Variables|Default|GetIsHightActive))
      (Default|CallOnLowValue)
      (Variables|Default|SetIsHightActive false))))

(event EventBeginPlay
  (bind _returnvalue (Utilities|Time|SetTimerbyEvent (delegate Custom|UpdateValue) 2.0 true))
  (Variables|Default|SetTimerHandle _returnvalue)
  (bind _returnvalue_2 (Utilities|Time|SetTimerbyEvent (delegate Custom|Update) 0.1 true))
  (Variables|Default|SetValueDown _returnvalue_2))

(event EventPostLogin
  (params (NewPlayer :type Player%20Controller%20Object%20Reference))
  (Default|AddNewPlayer (CallFunction|GetCustomGameState) (Variables|/Script/Engine.Controller|GetPlayerState NewPlayer))
  (Utilities|FlowControl|DoOnce false
    (:Completed
      (bind _returnvalue (Utilities|Time|SetTimerbyEvent (delegate Custom|Time) 1.0 true))
      (Variables|Default|SetTimeUpdate _returnvalue)
      (Utilities|FlowControl|Delay 1.0)
      (for _index (range 0 4)
        (CallFunction|SpawmActor)))))

(fn ConstructionScript)

(fn GetAudioValue
  (return (Variables|Default|GetAudioValue)))

(fn SpawmActor
  (bind _returnvalue (Subsystems|GetSpawnSubsystem))
  (bind _returnvalue_2 (Class|SpawnSubsystem|GetCount _returnvalue))
  (LocalVariables|SetNum _returnvalue_2)
  (LocalVariables|SetRandomID (Math|Random|RandomInteger (- _returnvalue_2 1)))
  (LocalVariables|SetRandomID (Math|Integer|%(Integer) (+ (LocalVariables|GetRandomID) 1) (LocalVariables|GetNum)) :!label _label)
  (bind _output_get (LocalVariables|SetLocalActor (Class|SpawnSubsystem|GetActor (Subsystems|GetSpawnSubsystem) (LocalVariables|GetRandomID))))
  (Utilities|IsValid _output_get
    (:Is%20Valid
      (bind _asbp_base_interaction (Utilities|Casting|CastToBP_BaseInteraction (LocalVariables|GetLocalActor))
        (:then
          (if (and (Variables|/Game/Game/Components/Interaction/BP_BaseInteraction.BP_BaseInteraction_C|GetIsSpawnKey _asbp_base_interaction) (== (Class|SceneComponent|GetNumChildrenComponents (Variables|/Game/Game/Components/Interaction/BP_BaseInteraction.BP_BaseInteraction_C|GetSpawnPoint _asbp_base_interaction)) 0))
            (bind _returnvalue_3 (Game|SpawnActorfromClass "/Game/Game/Actors/Interactions/BP_Key.BP_Key_C" (Math|Transform|MakeTransform "0, 0, 0" "0, 0, 0" "1.000000,1.000000,1.000000") "Undefined" "MultiplyWithRoot" 0 0))
            (Transformation|AttachComponentToComponent _returnvalue_3 (Variables|/Game/Game/Components/Interaction/BP_BaseInteraction.BP_BaseInteraction_C|GetSpawnPoint _asbp_base_interaction) "None" "KeepRelative" "KeepRelative" "KeepRelative" true)
            (else
              (goto _label))))
        (:CastFailed
          (goto _label))))
    (:Is%20Not%20Valid
      (goto _label))))

(fn GetCustomGameState
  (Utilities|IsValid (Variables|Default|GetGameGS)
    (:Is%20Valid
      _)
    (:Is%20Not%20Valid
      (bind _asbp_game_gs (Utilities|Casting|CastToBP_GameGS (Game|GetGameState)))
      (Variables|Default|SetGameGS _asbp_game_gs)))
  (return (Variables|Default|GetGameGS)))