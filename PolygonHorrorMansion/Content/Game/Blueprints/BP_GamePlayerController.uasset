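; Networked player controller that bridges the game mode and each client's UI, and handles look input and viewer switching.
; On authority it relays game mode audio value, time, key and game-end events through client calls to dispatchers and the HUD.
; Remote clients play sound subsystem sounds, send their values to the server, and decay the audio value on a timer.
; Keys 1 and 2 cycle the view target through other PlayerArray pawns.
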(event Custom|CustomEvent
  (Variables|Default|SetAudioValue (Math|Float|Clamp(Float) (- (Variables|Default|GetAudioValue) 0.005))))

(event Custom|CustomEvent_0
  (params (AudioValue :type Float%20%28double-precision%29))
  ;[0.15 0.15 0.15 0.5] Comment
  (CallFunction|Client|SetValue AudioValue))

(event Custom|Client%20|%20TimeUpdate
  (params (Time :type Integer))
  ;[0.15 0.15 0.15 0.5] Comment
  (Default|CallOnTimeUpdate Time))

(event Custom|Client%20|%20UpdateKeys
  (params (Keys :type Integer))
  ;[0.15 0.15 0.15 0.5] Comment
  (Default|CallOnKeysUpdate Keys))

(event Custom|UpdateKeys
  (params (CurrentKeys :type Integer))
  ;[0.15 0.15 0.15 0.5] Comment
  (CallFunction|Client|UpdateKeys CurrentKeys))

(event Custom|GameEnd
  (params (IsSuccess :type Boolean))
  ;[0.15 0.15 0.15 0.5] Comment
  (CallFunction|Client|EndGame IsSuccess))

(event Custom|Client%20|%20EndGame
  (params (IsSuccess :type Boolean))
  ;[0.15 0.15 0.15 0.5] Comment
  (Default|CreateEndGame (Variables|Default|GetGame%20HUD) IsSuccess))

(event Custom|Client%20|%20SetValue
  (params (Value :type Float%20%28double-precision%29))
  ;[0.15 0.15 0.15 0.5] Comment
  (Variables|Default|SetAudioValue Value))

(event Custom|CustomEvent_1
  (params (Sound :type Sound%20Base%20Object%20Reference) (Location :type Vector) (Value :type Float%20%28single-precision%29))
  (Audio|PlaySoundatLocation Sound Location "0, 0, 0" 1.0 1.0 0.0 0 0 0 0)
  (CallFunction|Server|SetValue Value))

(event Custom|Server%20|%20SetValue
  (params (Value :type Float%20%28double-precision%29))
  ;[0.15 0.15 0.15 0.5] Comment
  (Default|SetValue (Variables|Default|GetServer%20|%20GM) Value))

(event Custom|SetInteracted
  (params (IsInteracted :type Boolean))
  ;[0.15 0.15 0.15 0.5] Comment
  (Default|SetInteract (Variables|/Game/Game/UI/HUD/BP_GameHUD.BP_GameHUD_C|GetGameWidget (Variables|Default|GetGame%20HUD)) IsInteracted))

(event Custom|ViewClient
  (params (ID :type Integer))
  (bind _output_get (Variables|Default|SetViewTarget (PlayerState|GetPawn (Utilities|Array|Get(acopy) (Variables|/Script/Engine.GameStateBase|GetPlayerArray (Game|GetGameState)) ID))))
  (Game|Player|SetViewTargetwithBlend _output_get 0.0 "VTBlend_Linear" 0.0 false))

(event Custom|NextViewer
  ;[0.15 0.15 0.15 0.5] Comment
  (if (== (Math|Integer|%(Integer) (+ (Variables|Default|GetViewClientID) 1) (Utilities|Array|Length (Variables|/Script/Engine.GameStateBase|GetPlayerArray (Game|GetGameState)))) 0)
    (Variables|Default|SetViewClientID 1)
    (else
      (Variables|Default|SetViewClientID (Math|Integer|%(Integer) (+ (Variables|Default|GetViewClientID) 1) (Utilities|Array|Length (Variables|/Script/Engine.GameStateBase|GetPlayerArray (Game|GetGameState)))))))
  (CallFunction|ViewClient (Variables|Default|GetViewClientID)))

(event Custom|PrevViewer
  (if (== (+ (- (Variables|Default|GetViewClientID) 1) (select (< (- (Variables|Default|GetViewClientID) 1) 0) (Utilities|Array|Length (Variables|/Script/Engine.GameStateBase|GetPlayerArray (Game|GetGameState))) 0)) 0)
    (Variables|Default|SetViewClientID 1)
    (else
      (Variables|Default|SetViewClientID (+ (- (Variables|Default|GetViewClientID) 1) (select (< (- (Variables|Default|GetViewClientID) 1) 0) (Utilities|Array|Length (Variables|/Script/Engine.GameStateBase|GetPlayerArray (Game|GetGameState))) 0)))))
  (CallFunction|ViewClient (Variables|Default|GetViewClientID)))

(event Custom|CustomEvent_2
  (params (Time :type Integer))
  ;[0.15 0.15 0.15 0.5] Comment
  (CallFunction|Client|TimeUpdate Time))

(event Input|EnhancedActionEvents|EnhancedInputActionIA_LookRL
  (params (ActionValue :type Float%20%28double-precision%29) (ElapsedSeconds :type Float%20%28double-precision%29) (TriggeredSeconds :type Float%20%28double-precision%29) (InputAction :type Input%20Action%20Object%20Reference :default "/Game/Game/Input/Actions/IA_LookRL.IA_LookRL"))
  (bind _returnvalue (Pawn|GetControlledPawn))
  ;[0.15 0.15 0.15 0.5] Comment
  (Utilities|IsValid _returnvalue
    (:Is%20Valid
      (Pawn|Input|AddControllerYawInput _returnvalue ActionValue))))

(event Input|EnhancedActionEvents|EnhancedInputActionIA_LookUD
  (params (ActionValue :type Float%20%28double-precision%29) (ElapsedSeconds :type Float%20%28double-precision%29) (TriggeredSeconds :type Float%20%28double-precision%29) (InputAction :type Input%20Action%20Object%20Reference :default "/Game/Game/Input/Actions/IA_LookUD.IA_LookUD"))
  (bind _returnvalue (Pawn|GetControlledPawn))
  ;[0.15 0.15 0.15 0.5] Comment
  (Utilities|IsValid _returnvalue
    (:Is%20Valid
      (Pawn|Input|AddControllerPitchInput _returnvalue ActionValue))))

(event EventBeginPlay
  (CallFunction|SetInputMapping)
  (Networking|SwitchHasAuthority
    (:Authority
      ;[0.15 0.15 0.15 0.5] Comment
      (bind _asbp_game_gm (Utilities|Casting|CastToBP_GameGM (Game|GetGameMode)))
      (bind _output_get (Variables|Default|SetServer%20|%20GM _asbp_game_gm))
      (EventDispatchers|BindEventtoOnValueUpdate _output_get (delegate Custom|CustomEvent_0))
      (EventDispatchers|BindEventtoOnTimeUpdate (Variables|Default|GetServer%20|%20GM) (delegate Custom|CustomEvent_2))
      (EventDispatchers|BindEventtoOnUpdateKey (Variables|Default|GetServer%20|%20GM) (delegate Custom|UpdateKeys))
      (EventDispatchers|BindEventtoOnGameEnd (Variables|Default|GetServer%20|%20GM) (delegate Custom|GameEnd)))
    (:Remote
      (bind _returnvalue (Utilities|Time|SetTimerbyEvent (delegate Custom|CustomEvent) 0.1 true))
      (Variables|Default|SetNewVar _returnvalue)
      (EventDispatchers|BindEventtoOnPlaySoundDelegate (Subsystems|GetSoundSubsystem) (delegate Custom|CustomEvent_1))
      (bind _asbp_game_hud (Utilities|Casting|CastToBP_GameHUD (HUD|GetHUD)))
      (Variables|Default|SetGame%20HUD _asbp_game_hud))))

(event Input|KeyboardEvents|2
  (params (Key :type Key%20Structure :default "None"))
  (:Pressed
    (CallFunction|NextViewer)
    (Development|PrintString (Utilities|String|ToString(Integer) (Variables|Default|GetViewClientID)))))

(event Input|KeyboardEvents|1
  (params (Key :type Key%20Structure :default "None"))
  (:Pressed
    (CallFunction|PrevViewer)
    (Development|PrintString (Utilities|String|ToString(Integer) (Variables|Default|GetViewClientID)))))

(fn ConstructionScript)

(fn SetInputMapping
  (bind _returnvalue (PlayerController|LocalPlayerSubsystems|GetEnhancedInputLocalPlayerSubsystem))
  (Utilities|IsValid _returnvalue
    (:Is%20Valid
      (Input|AddMappingContext _returnvalue "/Game/Game/Input/IMC_Game.IMC_Game" 0 "(bIgnoreAllPressedKeysUntilRelease=True,bForceImmediately=False,bNotifyUserSettings=False)"))))

(fn GetController
  (for _array_element (Variables|/Script/Engine.GameStateBase|GetPlayerArray (Game|GetGameState))
    (if (== (Utilities|Array|FindItem (Variables|/Script/Engine.Actor|GetTags _array_element) "Dead") -1)
      (return (Game|GetPlayerController _array_element)))))